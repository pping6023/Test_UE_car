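; Checkpoint actor for lap counting that moves a single trigger box along eight checkpoint positions, Cp1 to Cp8.
; Each overlap moves the box to the transform indexed by CPCount and increments the count, with a one-second DoOnce lockout against repeat triggers.
; When the count reaches eight, a short delay precedes resetting it, incrementing LAP, and returning the box to Cp1 while LAP is within MaxLaps.
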(event OnComponentBeginOverlap(CP_Triggerbox)
  (params (OverlappedComponent :type Primitive%20Component%20Object%20Reference) (OtherActor :type Actor%20Object%20Reference) (OtherComp :type Primitive%20Component%20Object%20Reference) (OtherBodyIndex :type Integer) (bFromSweep :type Boolean) (SweepResult :type Hit%20Result%20Structure%20%28by%20ref%29))
  (if (== (Variables|Default|GetCP_Count) 8)
    (Utilities|FlowControl|Delay 0.2)
    (Variables|Default|SetCP_Count 1)
    (Variables|Default|SetLAP (+ (Variables|Default|GetLAP) 1))
    (if (<= (Variables|Default|GetLAP) (Variables|Default|GetMaxLaps))
      ;[1 1 1] 체크포인트 시작점으로 이동
      (Transformation|SetWorldTransform (Variables|Default|GetCP_Triggerbox) (Transformation|GetWorldTransform (Variables|Default|Getcp_1)) false false))
    (else
      (Utilities|FlowControl|DoOnce false :!label _label
        (:Completed
          (Transformation|SetWorldTransform (Variables|Default|GetCP_Triggerbox) (Transformation|GetWorldTransform (Utilities|Array|Get(acopy) (Utilities|Array|MakeArray (Variables|Default|Getcp_1) (Variables|Default|Getcp_2) (Variables|Default|Getcp_3) (Variables|Default|Getcp_4) (Variables|Default|Getcp_5) (Variables|Default|Getcp_6) (Variables|Default|Getcp_7) (Variables|Default|Getcp_8)) (Variables|Default|GetCP_Count))) false false)
          (Variables|Default|SetCP_Count (+ (Variables|Default|GetCP_Count) 1))
          (Utilities|FlowControl|Delay 1.0)
          (goto _label Reset))))))

(event EventBeginPlay)

(event Collision|EventActorBeginOverlap
  (params (OtherActor :type Actor%20Object%20Reference)))

(event EventTick
  (params (DeltaSeconds :type Float%20%28single-precision%29)))

(fn ConstructionScript)